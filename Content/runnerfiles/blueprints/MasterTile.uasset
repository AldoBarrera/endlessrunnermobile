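; Endless-runner track tile that fills three lanes with random obstacles and pickups and extends the track as the player passes.
; BeginPlay runs Spawn2, a cascade of fresh random rolls per lane, where an empty lane ends the chain for later lanes.
; Character overlap with the box has ThirdPersonGameMode spawn another tile, adds multiplied points, raises clamped walk speed, then destroys the tile after a delay.
; The older Spawnobstacles function is unused.
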(event OnComponentBeginOverlap(Box)
  (params (OverlappedComponent :type Primitive%20Component%20Object%20Reference) (OtherActor :type Actor%20Object%20Reference) (OtherComp :type Primitive%20Component%20Object%20Reference) (OtherBodyIndex :type Integer) (bFromSweep :type Boolean) (SweepResult :type Hit%20Result%20Structure%20%28by%20ref%29))
  (Utilities|Casting|CastToThirdPersonCharacter OtherActor)
  (bind _asthird_person_game_mode (Utilities|Casting|CastToThirdPersonGameMode (Game|GetGameMode)))
  (Default|Spawntile _asthird_person_game_mode)
  (bind _asthird_person_game_mode_2 (Utilities|Casting|CastToThirdPersonGameMode (Game|GetGameMode)))
  (bind _output_get (Variables|/Game/ThirdPersonBP/Blueprints/ThirdPersonGameMode.ThirdPersonGameMode_C|Setcurrentpoints _asthird_person_game_mode_2 (+ (* 1 (Variables|/Game/ThirdPersonBP/Blueprints/ThirdPersonGameMode.ThirdPersonGameMode_C|Getpointsmultiplier _asthird_person_game_mode_2)) (Variables|/Game/ThirdPersonBP/Blueprints/ThirdPersonGameMode.ThirdPersonGameMode_C|Getcurrentpoints _asthird_person_game_mode_2))))
  (Development|PrintString (Utilities|String|ToString(Integer) _output_get))
  (bind _asthird_person_character (Utilities|Casting|CastToThirdPersonCharacter (Game|GetPlayerCharacter 0)))
  (Variables|/Script/Engine.CharacterMovementComponent|SetMaxWalkSpeed (Variables|/Script/Engine.Character|GetCharacterMovement _asthird_person_character) (Math|Float|Clamp(Float) (* (Variables|/Script/Engine.CharacterMovementComponent|GetMaxWalkSpeed (Variables|/Script/Engine.Character|GetCharacterMovement _asthird_person_character)) 1.01) 1e+02 1.2e+03))
  (Utilities|FlowControl|Delay 1.0)
  (Actor|DestroyActor))

(event EventBeginPlay
  (CallFunction|Spawn2))

(event Collision|EventActorBeginOverlap
  (params (OtherActor :type Actor%20Object%20Reference)))

(event EventTick
  (params (DeltaSeconds :type Float%20%28single-precision%29)))

(fn ConstructionScript)

(fn Spawnobstacles
  (bind _lane0 (Variables|Default|Getlane0))
  (bind _lane1 (Variables|Default|Getlane1))
  (bind _lane2 (Variables|Default|Getlane2))
  (bind _returnvalue (Transformation|GetWorldTransform _lane2))
  (bind _returnvalue_2 (Transformation|GetWorldTransform _lane0))
  (bind _returnvalue_3 (Transformation|GetWorldTransform _lane1))
  ;[1 1 1] lane0
  (switch int (Math|Random|RandomIntegerinRange 0 4)
    (:1
      (Game|SpawnActorfromClass "/Game/runnerfiles/blueprints/obstacle_pipe.obstacle_pipe_C" _returnvalue_2 "Undefined" 0 0)
      ;[1 1 1] lane1
      (switch int (Math|Random|RandomIntegerinRange 0 4)
        (:1
          (Game|SpawnActorfromClass "/Game/runnerfiles/blueprints/obstacle_pipe.obstacle_pipe_C" _returnvalue_3 "Undefined" 0 0)
          ;[1 1 1] lane2
          (switch int (Math|Random|RandomIntegerinRange 0 4)
            (:1
              (Game|SpawnActorfromClass "/Game/runnerfiles/blueprints/obstacle_pipe.obstacle_pipe_C" _returnvalue "Undefined" 0 0))
            (:2
              (Game|SpawnActorfromClass "/Game/runnerfiles/blueprints/obstacle_box1.obstacle_box1_C" _returnvalue "Undefined" 0 0))
            (:3
              (Game|SpawnActorfromClass "/Game/runnerfiles/blueprints/coin_pickup.coin_pickup_C" _returnvalue "Undefined" 0 0))
            (:4
              (Game|SpawnActorfromClass "/Game/runnerfiles/blueprints/magnet_pickup.magnet_pickup_C" _returnvalue "Undefined" 0 0))))
        (:2
          (Game|SpawnActorfromClass "/Game/runnerfiles/blueprints/obstacle_box1.obstacle_box1_C" _returnvalue_3 "Undefined" 0 0))
        (:3
          (Game|SpawnActorfromClass "/Game/runnerfiles/blueprints/coin_pickup.coin_pickup_C" _returnvalue_3 "Undefined" 0 0))
        (:4
          (Game|SpawnActorfromClass "/Game/runnerfiles/blueprints/magnet_pickup.magnet_pickup_C" _returnvalue_3 "Undefined" 0 0))))
    (:2
      (Game|SpawnActorfromClass "/Game/runnerfiles/blueprints/obstacle_box1.obstacle_box1_C" _returnvalue_2 "Undefined" 0 0))
    (:3
      (Game|SpawnActorfromClass "/Game/runnerfiles/blueprints/coin_pickup.coin_pickup_C" _returnvalue_2 "Undefined" 0 0))
    (:4
      (Game|SpawnActorfromClass "/Game/runnerfiles/blueprints/magnet_pickup.magnet_pickup_C" _returnvalue_2 "Undefined" 0 0))))

(fn Spawn2
  (bind _returnvalue (Math|Random|RandomFloatinRange 0.0 1.0))
  (bind _returnvalue_2 (Math|Random|RandomFloatinRange 0.0 1.0))
  (bind _returnvalue_3 (Math|Random|RandomFloatinRange 0.0 1.0))
  (bind _lane0 (Variables|Default|Getlane0))
  (bind _lane1 (Variables|Default|Getlane1))
  (bind _lane2 (Variables|Default|Getlane2))
  (bind _returnvalue_4 (Transformation|GetWorldTransform _lane1))
  (bind _returnvalue_5 (Transformation|GetWorldTransform _lane2))
  (bind _returnvalue_6 (Transformation|GetWorldTransform _lane0))
  (if (Math|Float|InRange(Float) _returnvalue_3 0.0 0.4)
    (Game|SpawnActorfromClass "/Game/runnerfiles/blueprints/obstacle_pipe.obstacle_pipe_C" _returnvalue_6 "Undefined" 0 0)
    (if (Math|Float|InRange(Float) _returnvalue_2 0.0 0.4) :!label _label
      (Game|SpawnActorfromClass "/Game/runnerfiles/blueprints/obstacle_pipe.obstacle_pipe_C" _returnvalue_4 "Undefined" 0 0)
      (if (Math|Float|InRange(Float) _returnvalue 0.0 0.4) :!label _label_2
        (Game|SpawnActorfromClass "/Game/runnerfiles/blueprints/obstacle_pipe.obstacle_pipe_C" _returnvalue_5 "Undefined" 0 0)
        (elif (Math|Float|InRange(Float) _returnvalue 0.4 0.5)
          (Game|SpawnActorfromClass "/Game/runnerfiles/blueprints/obstacle_box1.obstacle_box1_C" _returnvalue_5 "Undefined" 0 0)
          (elif (Math|Float|InRange(Float) _returnvalue 0.5 0.9)
            (Game|SpawnActorfromClass "/Game/runnerfiles/blueprints/coin_pickup.coin_pickup_C" _returnvalue_5 "Undefined" 0 0)
            (elif (Math|Float|InRange(Float) _returnvalue 0.9 1.0)
              (Game|SpawnActorfromClass "/Game/runnerfiles/blueprints/magnet_pickup.magnet_pickup_C" _returnvalue_5 "Undefined" 0 0)
              (elif (Math|Float|InRange(Float) 0.0 0.975 1.0)
                (Game|SpawnActorfromClass "/Game/runnerfiles/blueprints/boots_pickup1.boots_pickup1_C" _returnvalue_5 "Undefined" 0 0))))))
      (elif (Math|Float|InRange(Float) _returnvalue_2 0.4 0.5)
        (Game|SpawnActorfromClass "/Game/runnerfiles/blueprints/obstacle_box1.obstacle_box1_C" _returnvalue_4 "Undefined" 0 0)
        (goto _label_2)
        (elif (Math|Float|InRange(Float) _returnvalue_2 0.5 0.9)
          (Game|SpawnActorfromClass "/Game/runnerfiles/blueprints/coin_pickup.coin_pickup_C" _returnvalue_4 "Undefined" 0 0)
          (goto _label_2)
          (elif (Math|Float|InRange(Float) _returnvalue_2 0.9 1.0)
            (Game|SpawnActorfromClass "/Game/runnerfiles/blueprints/magnet_pickup.magnet_pickup_C" _returnvalue_4 "Undefined" 0 0)
            (goto _label_2)
            (elif (Math|Float|InRange(Float) _returnvalue_2 0.975 1.0)
              (Game|SpawnActorfromClass "/Game/runnerfiles/blueprints/boots_pickup1.boots_pickup1_C" _returnvalue_4 "Undefined" 0 0)
              (goto _label_2))))))
    (elif (Math|Float|InRange(Float) _returnvalue_3 0.4 0.5)
      (Game|SpawnActorfromClass "/Game/runnerfiles/blueprints/obstacle_box1.obstacle_box1_C" _returnvalue_6 "Undefined" 0 0)
      (goto _label)
      (elif (Math|Float|InRange(Float) _returnvalue_3 0.5 0.9)
        (Game|SpawnActorfromClass "/Game/runnerfiles/blueprints/coin_pickup.coin_pickup_C" _returnvalue_6 "Undefined" 0 0)
        (goto _label)
        (elif (Math|Float|InRange(Float) _returnvalue_3 0.95 0.975)
          (Game|SpawnActorfromClass "/Game/runnerfiles/blueprints/magnet_pickup.magnet_pickup_C" _returnvalue_6 "Undefined" 0 0)
          (goto _label)
          (elif (Math|Float|InRange(Float) _returnvalue_3 0.975 1.0)
            (Game|SpawnActorfromClass "/Game/runnerfiles/blueprints/boots_pickup1.boots_pickup1_C" _returnvalue_6 "Undefined" 0 0)
            (goto _label)))))))